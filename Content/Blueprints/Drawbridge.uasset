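; Drawbridge actor that the player opens and closes with the Action input, which is enabled while something overlaps it, alongside a "Press F" debug print.
; Each press flips IsClosed and plays or reverses the Drawbridge timeline, which drives the roll of the bridge mesh.
; Every Tick, both chain cables take length and material tiling from the distance between Cable and Scene, then toggle visibility to force a re-render.
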(event Collision|EventActorEndOverlap
  (params (OtherActor :type Actor%20Object%20Reference))
  ;[1 1 1] Drawbridge Controls
  (Input|DisableInput (Game|GetPlayerController 0)))

(event EventTick
  (params (DeltaSeconds :type Float%20%28single-precision%29))
  (bind _scene (Variables|Default|GetScene))
  (bind _cable (Variables|Default|GetCable))
  (bind _cable_2 (Variables|Default|GetCable))
  (bind _cable1 (Variables|Default|GetCable1))
  (bind _returnvalue (Transformation|GetWorldLocation _scene))
  (bind _returnvalue_2 (Transformation|GetWorldLocation _cable))
  (bind _returnvalue_3 (- _returnvalue_2 _returnvalue))
  (bind _returnvalue_4 (Math|Vector|VectorLength _returnvalue_3))
  ;[1 1 1] Chain
  (bind _output_get (Variables|/Script/CableComponent.CableComponent|SetCableLength (Variables|Default|GetCable) (* _returnvalue_4 0.9)))
  (Variables|/Script/CableComponent.CableComponent|SetCableLength (Variables|Default|GetCable1) _output_get)
  (bind _output_get_2 (Variables|/Script/CableComponent.CableComponent|SetTileMaterial (Variables|Default|GetCable) (/ _returnvalue_4 5e+01)))
  (Variables|/Script/CableComponent.CableComponent|SetTileMaterial _cable1 _output_get_2)
  ;;[1 1 1] Re-render Cables
  (Rendering|SetVisibility _cable1 false false)
  (Rendering|SetVisibility _cable1 true false)
  (Rendering|SetVisibility _cable_2 false false)
  (Rendering|SetVisibility _cable_2 true false))

(event Collision|EventActorBeginOverlap
  (params (OtherActor :type Actor%20Object%20Reference))
  ;[1 1 1] Drawbridge Controls
  (Input|EnableInput (Game|GetPlayerController 0))
  (Development|PrintString "Press F"))

(event Input|ActionEvents|InputActionAction
  (params (Key :type Key%20Structure))
  ;[1 1 1] Drawbridge Controls
  (:Pressed
    (if (Variables|Default|GetIsClosed)
      (Variables|Default|SetIsClosed false)
      (bind _rotation (Timeline|Drawbridge Play)
        (:Update
          (Transformation|SetRelativeRotation (Variables|Default|GetDrawbridgeBridge_mesh) (Math|Rotator|MakeRotator _rotation 0.0 0.0) false false)))
      (else
        (Variables|Default|SetIsClosed true)
        (Timeline|Drawbridge Reverse)))))

(fn ConstructionScript)