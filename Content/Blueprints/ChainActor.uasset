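; ChainActor is a construction-time actor that builds a straight chain of static meshes from its location toward an EndPoint offset.
; The construction script rotates the Cube component in world space to face that offset, treating EndPoint as world-axis relative to the actor.
; It then adds mesh components every 100 units along X, covering the vector's length, and attaches them to Cube.
; The event graph has no runtime logic.
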(event EventBeginPlay)

(event Collision|EventActorBeginOverlap
  (params (OtherActor :type Actor%20Object%20Reference)))

(event EventTick
  (params (DeltaSeconds :type Float%20%28single-precision%29)))

(fn ConstructionScript
  (bind _returnvalue (Transformation|GetActorLocation))
  (Transformation|SetWorldRotation (Variables|Default|GetCube) (Math|Rotator|FindLookatRotation _returnvalue (+ _returnvalue (Variables|Default|GetEndPoint))) false false)
  (for _index (range 0 (Math|Float|Floor (/ (Math|Vector|VectorLength (Variables|Default|GetEndPoint)) 1e+02)))
    (bind _returnvalue_2 (AddComponent|AddStaticMeshComponent false (Math|Transform|MakeTransform (Math|Vector|MakeVector (* _index 1e+02) 0.0 0.0) "0, 0, 0" "1.000000,1.000000,1.000000")))
    (Transformation|AttachComponentToComponent _returnvalue_2 (Variables|Default|GetCube) "None" "KeepRelative" "KeepRelative" "KeepRelative" true)))